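; BP_SlingshotRock is the rock actor for an enemy slingshot ability, adding a random tumbling spin to its mesh.
; BeginPlay picks independent random pitch, yaw and roll rates, each either positive or negative.
; Tick applies those rates, scaled by delta time, as local rotation on RockMesh.
; The graph holds only this cosmetic spin, with no movement or hit logic.
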(event EventBeginPlay
  (Utilities|FlowControl|Sequence
    (:then_0
      (Variables|Default|SetPitchRotationRate (Math|Random|RandomFloatinRange -5e+02 5e+02)))
    (:then_1
      (Variables|Default|SetYawRotationRate (Math|Random|RandomFloatinRange -5e+02 5e+02)))
    (:then_2
      (Variables|Default|SetRollRotationRate (Math|Random|RandomFloatinRange -5e+02 5e+02)))))

(event Collision|EventActorBeginOverlap
  (params (OtherActor :type Actor%20Object%20Reference)))

(event EventTick
  (params (DeltaSeconds :type Float%20%28single-precision%29))
  (Transformation|AddLocalRotation (Variables|Default|GetRockMesh) (Math|Rotator|MakeRotator (* (Variables|Default|GetRollRotationRate) DeltaSeconds) (* (Variables|Default|GetPitchRotationRate) DeltaSeconds) (* (Variables|Default|GetYawRotationRate) DeltaSeconds)) false false))

(fn ConstructionScript)