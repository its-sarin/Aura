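; Enemy ranged attack gameplay ability that fires a projectile at the avatar's combat target.
; On activation it turns the avatar toward the target, caches that location and plays a random tagged attack montage.
; The montage's gameplay event tag times the shot: a debug sphere marks the matching combat socket and the projectile spawns toward the cached location.
; The ability ends shortly after firing, leaving the montage playing.
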(event Ability|EventActivateAbility
  (bind _returnvalue (Ability|GetAvatarActorfromActorInfo))
  (bind _returnvalue_2 (Class|EnemyInterface|GetCombatTarget(Message) _returnvalue))
  (Class|CombatInterface|UpdateFacingTarget(Message) _returnvalue (Transformation|GetActorLocation _returnvalue_2))
  (Variables|Default|SetProjectileTargetLocation (Transformation|GetActorLocation _returnvalue_2))
  (bind _returnvalue_3 (Class|CombatInterface|GetAttackMontages(Message) (Ability|GetAvatarActorfromActorInfo)))
  (bind _output_get (Variables|Default|SetTaggedMontage (Class|AuraDamageGameplayAbility|GetRandomTaggedMontagefromArray _returnvalue_3)))
  (|PlayMontageandWaitProxy "None" (.Montage (Utilities|Struct|BreakTaggedMontage _output_get)) 1.0 "None" false 1.0 0.0 false
    (:then
      (Ability|Tasks|WaitGameplayEvent (.MontageTag (Utilities|Struct|BreakTaggedMontage _output_get)) 0
        (:EventReceived
          (bind _returnvalue_4 (Class|CombatInterface|GetCombatSocketLocation(Message) (Ability|GetAvatarActorfromActorInfo) (.MontageTag (Utilities|Struct|BreakTaggedMontage _output_get))))
          (Rendering|Debug|DrawDebugSphere _returnvalue_4 2e+01 12 "(R=1.000000,G=0.904668,B=0.000000,A=1.000000)" 0.5)
          (Class|AuraProjectileSpell|SpawnProjectile (Variables|Default|GetProjectileTargetLocation))
          (Utilities|FlowControl|Delay 0.5)
          (Ability|EndAbility))))))

(event Ability|EventOnEndAbility
  (params (bWasCancelled :type Boolean)))