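; GA_MeleeAttack is a melee attack ability that turns the avatar toward its combat target and plays the goblin spear attack montage.
; On the montage's melee gameplay event, it gathers live players within a small radius of the combat socket, ignoring the avatar.
; Hits are only visualized with debug spheres, with no damage applied yet.
; The ability ends after that check, or when the montage completes, is interrupted or is cancelled.
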(event Ability|EventActivateAbility
  (bind _returnvalue (Ability|GetAvatarActorfromActorInfo))
  (bind _returnvalue_2 (Ability|GetAvatarActorfromActorInfo))
  (bind _returnvalue_3 (Class|EnemyInterface|GetCombatTarget(Message) _returnvalue_2))
  (bind _ascombat_interface (Utilities|Casting|CastToCombatInterface _returnvalue_2))
  (Class|CombatInterface|UpdateFacingTarget _ascombat_interface (Transformation|GetActorLocation _returnvalue_3))
  (|PlayMontageandWaitProxy "None" "/Game/Assets/Enemies/Goblin/Animations/Spear/AM_Attack_GoblinSpear.AM_Attack_GoblinSpear" 1.0 "None" true 1.0 0.0 false
    (:then
      (Ability|Tasks|WaitGameplayEvent "(TagName=\"Event.Montage.Attack.Melee\")" 0
        (:EventReceived
          (bind _returnvalue_4 (Class|CombatInterface|GetCombatSocketLocation(Message) _returnvalue))
          (bind _outoverlappingactors (Class|AuraAbilitySystemLibrary|GetLivePlayersWithinRadius _returnvalue (Utilities|Array|MakeArray _returnvalue) _returnvalue_4 45.0))
          (for _array_element _outoverlappingactors
            (Rendering|Debug|DrawDebugSphere (Transformation|GetActorLocation _array_element) 45.0 12 "(R=0.000000,G=1.000000,B=0.582609,A=1.000000)" 1.0))
          (Ability|EndAbility))))
    (:OnCompleted
      (Ability|EndAbility :!label _label))
    (:OnInterrupted
      (goto _label))
    (:OnCancelled
      (goto _label))))

(event Ability|EventOnEndAbility
  (params (bWasCancelled :type Boolean)))