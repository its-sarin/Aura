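; Flame pillar actor that makes its fire light flicker continuously during play.
; From BeginPlay, it randomly picks one of two intensity timelines to play, and picks again whenever one finishes, so the flicker pattern varies.
; Each timeline update multiplies the curve value by a base intensity and applies it to the FireLight component.
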(event Custom|StartTimeline_1
  (bind _pointlightintensity (Timeline|FlameIntensity_1 PlayFromStart)
    (:Update
      (CallFunction|ScaleFlameIntensity _pointlightintensity))
    (:Finished
      (CallFunction|ChooseTimeline))))

(event Custom|StartTimeline_2
  (bind _pointlightintensity (Timeline|FlameIntensity_2 PlayFromStart)
    (:Update
      (CallFunction|ScaleFlameIntensity _pointlightintensity))
    (:Finished
      (CallFunction|ChooseTimeline))))

(event Custom|ChooseTimeline
  (switch int (Math|Random|RandomInteger 2)
    (:Default
      (CallFunction|StartTimeline2 :!label _label))
    (:0
      (CallFunction|StartTimeline1))
    (:1
      (goto _label))))

(event EventBeginPlay
  (CallFunction|ChooseTimeline))

(fn ConstructionScript)

(fn ScaleFlameIntensity
  (params (Intensity :type Float%20%28double-precision%29))
  (Rendering|Components|Light|SetIntensity (Variables|Default|GetFireLight) (* Intensity (Variables|Default|GetBaseIntensity))))